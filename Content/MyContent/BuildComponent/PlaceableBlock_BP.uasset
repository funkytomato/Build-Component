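; PlaceableBlock_BP is a buildable block that starts as a placement preview and becomes solid when placed.
; On BeginPlay it stores the mesh's original material, swaps in a preview material and disables collision.
; The Placed event restores the stored material and enables query and physics collision.
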(event Custom|Placed
  (Rendering|Material|SetMaterial (Variables|Default|GetStaticMesh) 0 (Variables|Default|GetDefaultMaterial))
  (Collision|SetCollisionEnabled (Variables|Default|GetStaticMesh) "QueryAndPhysics"))

(event EventBeginPlay
  (Variables|Default|SetDefaultMaterial (Rendering|Material|GetMaterial (Variables|Default|GetStaticMesh) 0))
  (Rendering|Material|SetMaterial (Variables|Default|GetStaticMesh) 0 "/Game/MyContent/BuildComponent/M_PreviewMaterial.M_PreviewMaterial")
  (Collision|SetCollisionEnabled (Variables|Default|GetStaticMesh) "NoCollision"))

(fn ConstructionScript)