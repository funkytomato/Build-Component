(event Custom|ResetBuild
  (Utilities|FlowControl|DoOnce false) ; enters at Reset
)

(event Custom|ToggleMenu
  (bind _returnvalue (Game|GetPlayerController 0))
  ;[1 1 1] Toggle Show Build Menu
  (bind _returnvalue_2 (Default|ToggleBuildMenu (Variables|Default|GetHUD)))
  (switch Utilities|FlowControl|Switch|SwitchonESlateVisibility _returnvalue_2
    (:Visible
      (Input|SetInputModeGameandUI _returnvalue 0 "DoNotLock" true false)
      (Variables|/Script/Engine.PlayerController|SetbShowMouseCursor _returnvalue true))
    (:Hidden
      (Input|SetInputModeGameOnly _returnvalue false)
      (Variables|/Script/Engine.PlayerController|SetbShowMouseCursor _returnvalue false))))

(event Input|EnhancedActionEvents|EnhancedInputActionIA_Build
  (params (ActionValue :type Boolean) (ElapsedSeconds :type Float%20%28double-precision%29) (TriggeredSeconds :type Float%20%28double-precision%29) (InputAction :type Input%20Action%20Object%20Reference :default "/Game/FirstPerson/Input/Actions/IA_Build.IA_Build"))
  ;[1 1 1] Build Placed Object
  (:Triggered
    (bind _buildpiece (Variables|Default|GetBuildPiece)
      (:then
        (Default|Placed _buildpiece)
        ;;[1 1 1] Remove this for continous building
        (Variables|PopupMenu|SetIsInBuildMode false)
        (Variables|Default|SetBuildPiece 0)
        (CallFunction|ResetBuild))
      (:else))))

(event Input|EnhancedActionEvents|EnhancedInputActionIA_Place
  (params (ActionValue :type Boolean) (ElapsedSeconds :type Float%20%28double-precision%29) (TriggeredSeconds :type Float%20%28double-precision%29) (InputAction :type Input%20Action%20Object%20Reference :default "/Game/FirstPerson/Input/Actions/IA_Place.IA_Place"))
  ;[1 1 1] Fire LineTrace to find Placeable area for Object
  (:Triggered
    (Variables|PopupMenu|SetIsInBuildMode true))
  (:Canceled
    (Variables|PopupMenu|SetIsInBuildMode false :!label _label))
  (:Completed
    (goto _label)))

(event Input|EnhancedActionEvents|EnhancedInputActionIA_ToggleMenu
  (params (ActionValue :type Boolean) (ElapsedSeconds :type Float%20%28double-precision%29) (TriggeredSeconds :type Float%20%28double-precision%29) (InputAction :type Input%20Action%20Object%20Reference :default "/Game/FirstPerson/Input/IA_ToggleMenu.IA_ToggleMenu"))
  (bind _returnvalue (Game|GetPlayerController 0))
  ;[1 1 1] Toggle Show Build Menu
  (:Started
    (bind _returnvalue_2 (Default|ToggleBuildMenu (Variables|Default|GetHUD)))
    (switch Utilities|FlowControl|Switch|SwitchonESlateVisibility _returnvalue_2
      (:Visible
        (Input|SetInputModeGameandUI _returnvalue 0 "DoNotLock" true false)
        (Variables|/Script/Engine.PlayerController|SetbShowMouseCursor _returnvalue true))
      (:Hidden
        (Input|SetInputModeGameOnly _returnvalue false)
        (Variables|/Script/Engine.PlayerController|SetbShowMouseCursor _returnvalue false)))))

(event EventBeginPlay
  ;[1 1 1] BeginPlay - Create Build Menu HUD
  (bind _returnvalue (UserInterface|CreateWidget "/Game/MyContent/BuildComponent/Interface/HeadsUpDisplay.HeadsUpDisplay_C"))
  (bind _output_get (Variables|Default|SetHUD _returnvalue))
  (UserInterface|Viewport|AddtoViewport _output_get 0))

(event EventTick
  (params (DeltaSeconds :type Float%20%28single-precision%29))
  (if (Variables|PopupMenu|GetIsInBuildMode)
    (Utilities|FlowControl|Sequence
      (:then_0
        (Utilities|FlowControl|DoOnce false
          (:Completed
            (bind _returnvalue (Game|SpawnActorfromClass (Variables|PopupMenu|GetBlockClass) (Transformation|GetActorTransform (Components|GetOwner)) "Undefined" 0 0))
            (Variables|Default|SetBuildPiece _returnvalue))))
      (:then_1
        (bind _out_hit_location (CallFunction|BuildTrace))
        (bind _buildpiece (Variables|Default|GetBuildPiece)
          (:then
            (Transformation|SetActorLocation _buildpiece (Class|KismetMathLibrary|VectorSnappedtoGrid _out_hit_location 1e+02) false false))
          (:else))))))

(fn BuildTrace
  (bind _returnvalue (Components|GetOwner))
  (bind _asbp_first_person_character (Utilities|Casting|CastToBP_FirstPersonCharacter _returnvalue))
  (bind _firstpersoncamera (Variables|/Game/MyContent/Character/BP_FirstPersonCharacter.BP_FirstPersonCharacter_C|GetFirstPersonCamera _asbp_first_person_character))
  (bind _returnvalue_2 (Transformation|GetWorldLocation _firstpersoncamera))
  (LocalVariables|SetIgnoredActors (Utilities|Array|MakeArray (Variables|Default|GetBuildPiece)))
  (bind (_outhit _returnvalue_3) (Collision|LineTraceByChannel _returnvalue_2 (+ _returnvalue_2 (* (Math|Vector|GetForwardVector _firstpersoncamera) 5e+02)) "TraceTypeQuery1" false (LocalVariables|GetIgnoredActors) "None"))
  (if _returnvalue_3
    (bind _outhit_2 (Collision|LineTraceByChannel (+ (.Location (Collision|BreakHitResult _outhit)) "0.000000,0.000000,500.000000") (- (.Location (Collision|BreakHitResult _outhit)) "0.000000,0.000000,50.000000") "TraceTypeQuery1" false (LocalVariables|GetIgnoredActors) "ForOneFrame"))
    (return (.location _outhit_2))
    (else
      (bind _outhit_3 (Collision|LineTraceByChannel (.TraceEnd (Collision|BreakHitResult _outhit)) (- (.TraceEnd (Collision|BreakHitResult _outhit)) "0.000000,0.000000,500.000000") "TraceTypeQuery1" false (LocalVariables|GetIgnoredActors) "ForOneFrame"))
      (return (.location _outhit_3)))))